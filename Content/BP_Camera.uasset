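; Top-down camera actor for a tile-based game, with screen-edge panning, mouse wheel zoom and tile picking under the cursor.
; It starts at a fixed height, pans each tick near viewport edges without delta-time scaling, and zooms by shifting its height.
; A per-tick deprojected mouse line trace, drawn for debugging, stores the hit Tile as CurrentTile, keeping the previous one on a miss.
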(event EventBeginPlay
  ;[1 1 1] Init position
  (Transformation|SetActorLocation "0.000000,0.000000,1000.000000" false false))

(event EventTick
  (params (DeltaSeconds :type Float%20%28single-precision%29))
  (bind _returnvalue (Game|GetPlayerState 0))
  (bind _returnvalue_2 (Game|GetPlayerController _returnvalue))
  (bind (_locationx _locationy) (Game|Player|GetMousePosition _returnvalue_2))
  (Variables|Default|SetMousePos (Math|Vector2D|MakeVector2D _locationx _locationy))
  (Variables|Default|SetViewportSize (Viewport|GetViewportSize))
  (Utilities|FlowControl|Sequence
    (:then_0
      ;[1 1 1] Camera Movement
      (Variables|Default|Setdirection "0, 0, 0")
      (Utilities|FlowControl|Sequence
        (:then_0
          (if (< (.x (Variables|Default|GetMousePos)) 5e+01)
            (Variables|Default|Setdirection "-1.000000,0.000000,0.000000")
            (elif (> (.x (Variables|Default|GetMousePos)) (- (.x (Variables|Default|GetViewportSize)) 5e+01))
              (Variables|Default|Setdirection "1.000000,0.000000,0.000000"))))
        (:then_1
          (if (< (.y (Variables|Default|GetMousePos)) 5e+01)
            (Variables|Default|Setdirection (+ (Variables|Default|Getdirection) "0.000000,-1.000000,0.000000"))
            (elif (> (.y (Variables|Default|GetMousePos)) (- (.y (Variables|Default|GetViewportSize)) 5e+01))
              (Variables|Default|Setdirection (+ (Variables|Default|Getdirection) "0.000000,1.000000,0.000000")))))
        (:then_2
          (Transformation|SetActorLocation (+ (Transformation|GetActorLocation) (* (Variables|Default|Getdirection) (Variables|Default|GetMoveSpeed))) false false))))
    (:then_1
      ;[1 1 1] Select tile
      (bind _outhit (Collision|LineTraceByChannel (.WorldPosition (Class|GameplayStatics|DeprojectScreentoWorld (Game|GetPlayerController 0) (Variables|Default|GetMousePos))) (+ (.WorldPosition (Class|GameplayStatics|DeprojectScreentoWorld (Game|GetPlayerController 0) (Variables|Default|GetMousePos))) (* (.WorldDirection (Class|GameplayStatics|DeprojectScreentoWorld (Game|GetPlayerController 0) (Variables|Default|GetMousePos))) 1e+05)) "TraceTypeQuery3" false 0 "ForOneFrame"))
      (bind _astile (Utilities|Casting|CastToTile (.HitActor (Collision|BreakHitResult _outhit))))
      (Variables|Default|SetCurrentTile _astile))))

(event Input|MouseEvents|LeftMouseButton
  (params (Key :type Key%20Structure :default "None")))

(event Input|MouseEvents|MouseWheelDown
  (params (Key :type Key%20Structure :default "None"))
  ;[1 1 1] Camera zoom
  (:Pressed
    (Transformation|SetActorLocation (+ (Transformation|GetActorLocation) (Math|Vector|MakeVector 0.0 0.0 (Math|Conversions|ToFloat(Integer) (Variables|Default|GetzoomOffset)))) false false)))

(event Input|MouseEvents|MouseWheelUp
  (params (Key :type Key%20Structure :default "None"))
  ;[1 1 1] Camera zoom
  (:Pressed
    (Transformation|SetActorLocation (- (Transformation|GetActorLocation) (Math|Vector|MakeVector 0.0 0.0 (Math|Conversions|ToFloat(Integer) (Variables|Default|GetzoomOffset)))) false false)))

(fn ConstructionScript)