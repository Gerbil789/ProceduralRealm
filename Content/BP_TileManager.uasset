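; BP_TileManager is a grid manager actor that spawns the tile grid and visualizes paths across it.
; The SpawnTiles event calls SpawnTileGrid with the row and column counts and a fixed spacing.
; DrawPath joins consecutive tile locations with short-lived, thick debug lines.
; An unconnected chain that gathers units, looks up their tiles and activates the first one never runs.
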(event Custom|SpawnTiles
  ;[1 1 1] Spawn grid
  (Class|TileManager|SpawnTileGrid (Variables|Default|GetNumRows) (Variables|Default|GetNumColumns) 2e+02))

(event EventBeginPlay)

(event Collision|EventActorBeginOverlap
  (params (OtherActor :type Actor%20Object%20Reference)))

(event EventTick
  (params (DeltaSeconds :type Float%20%28single-precision%29)))

(fn ConstructionScript)

(fn DrawPath
  (params (tiles :type Array%20of%20Tile%20Object%20References))
  (bind _output_get (LocalVariables|SetPath tiles))
  (LocalVariables|SetLast (Utilities|Array|Get(acopy) _output_get))
  (for _index (range 1 (- (Utilities|Array|Length (LocalVariables|GetPath)) 1))
    (Rendering|Debug|DrawDebugLine (.location (Transformation|GetActorTransform (LocalVariables|GetLast))) (.location (Transformation|GetActorTransform (Utilities|Array|Get(acopy) (LocalVariables|GetPath) _index))) "(R=0.000000,G=0.662919,B=1.000000,A=1.000000)" 2.0 2e+01)
    (LocalVariables|SetLast (Utilities|Array|Get(acopy) (LocalVariables|GetPath) _index))))