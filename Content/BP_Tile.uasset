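; BP_Tile is a tile actor that displays its Distance value as text and colors its plane by state.
; Construction creates a dynamic material instance, and SetColor writes the state's color to its Color parameter.
; Tick refreshes the text and picks the cursor-driven highlight first, then available or empty based on IsAvailable.
; Available and Occupied both use OccupiedColor, and Tick never selects Occupied.
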(event EventBeginPlay)

(event Collision|EventActorBeginOverlap
  (params (OtherActor :type Actor%20Object%20Reference)))

(event EventTick
  (params (DeltaSeconds :type Float%20%28single-precision%29))
  (Rendering|Components|TextRender|SetText (Variables|Default|GetTextRender) (Utilities|Text|ToText(Float) (Variables|GetDistance) "HalfToEven"))
  (if (Variables|Default|GetHighlight)
    (CallFunction|SetColor "Highlight")
    (elif (Class|SourceControlHelpers|IsAvailable)
      (CallFunction|SetColor "Available")
      (else
        (CallFunction|SetColor "Empty")))))

(event MouseInput|EventActorBeginCursorOver
  (Variables|Default|SetHighlight true))

(event MouseInput|EventActorEndCursorOver
  (Variables|Default|SetHighlight false))

(fn ConstructionScript
  (bind _returnvalue (Rendering|Material|CreateDynamicMaterialInstance (Variables|Default|GetPlane) 0 0 "None" :!class /Script/Engine.PrimitiveComponent))
  (Variables|Default|SetMaterial _returnvalue)
  (CallFunction|SetColor "Empty"))

(fn SetColor
  (params (color :type String))
  (switch string color
    (:Default
      (Development|PrintString "INVALID COLOR" true true "(R=1.000000,G=0.129130,B=0.000000,A=1.000000)" 1e+01))
    (:Empty
      (Rendering|Material|SetVectorParameterValue (Variables|Default|GetMaterial) "Color" (Variables|Default|GetEmptyColor) :!class /Script/Engine.MaterialInstanceDynamic))
    (:Available
      (Rendering|Material|SetVectorParameterValue (Variables|Default|GetMaterial) "Color" (Variables|Default|GetOccupiedColor) :!class /Script/Engine.MaterialInstanceDynamic))
    (:Occupied
      (Rendering|Material|SetVectorParameterValue (Variables|Default|GetMaterial) "Color" (Variables|Default|GetOccupiedColor) :!class /Script/Engine.MaterialInstanceDynamic))
    (:HighLIght
      (Rendering|Material|SetVectorParameterValue (Variables|Default|GetMaterial) "Color" (Variables|Default|GetHighlightColor) :!class /Script/Engine.MaterialInstanceDynamic))))