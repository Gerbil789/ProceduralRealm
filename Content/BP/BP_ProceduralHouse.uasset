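; BP_ProceduralHouse is an unfinished procedural house generator whose construction script is currently unwired.
; GeneratePoints walks a 3D grid set by Size and Offset, centered on X/Y and rising from zero in Z, keeping each cell at random against a Fill threshold.
; The disconnected nodes would store these points when Generate is set and loop over them, with a separate, unlinked static mesh component node.
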(event EventBeginPlay)

(event Collision|EventActorBeginOverlap
  (params (OtherActor :type Actor%20Object%20Reference)))

(event EventTick
  (params (DeltaSeconds :type Float%20%28single-precision%29)))

(fn ConstructionScript)

(fn GeneratePoints
  (LocalVariables|SetHalfwayX (/ (.x (Variables|Default|GetSize)) 2))
  (LocalVariables|SetHalfwayY (/ (.y (Variables|Default|GetSize)) 2))
  (for _index (range 0 (- (.x (Variables|Default|GetSize)) 1))
    (LocalVariables|SetCurrentX _index)
    (for _index_2 (range 0 (- (.y (Variables|Default|GetSize)) 1))
      (LocalVariables|SetCurrentY _index_2)
      (for _index_3 (range 0 (- (.z (Variables|Default|GetSize)) 1))
        (LocalVariables|SetCurrentZ _index_3)
        (if (<= (Math|Random|RandomFloatinRange 0.0 1.0) (Variables|Default|GetFill))
          (Utilities|Array|Add (LocalVariables|GetPointsArray) (Math|Vector|MakeVector (* (Variables|Default|GetOffset) (- (LocalVariables|GetCurrentX) (LocalVariables|GetHalfwayX))) (* (Variables|Default|GetOffset) (- (LocalVariables|GetCurrentY) (LocalVariables|GetHalfwayY))) (* (LocalVariables|GetCurrentZ) (Variables|Default|GetOffset))))))))
  (return (LocalVariables|GetPointsArray)))